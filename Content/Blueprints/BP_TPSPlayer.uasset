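; BP_TPSPlayer is the third-person player Blueprint, adding debug feedback to game-over and grenade events.
; OnGameOver calls its parent implementation and prints a message, while OnUsingGrenade prints its boolean flag.
; The sniper input event is empty; the nodes for creating and toggling the sniper UI with a camera FOV zoom are disconnected and never run.
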(event Input|EnhancedActionEvents|EnhancedInputActionIA_Sniper
  (params (ActionValue :type Boolean) (ElapsedSeconds :type Float%20%28double-precision%29) (TriggeredSeconds :type Float%20%28double-precision%29) (InputAction :type Input%20Action%20Object%20Reference :default "/Game/Input/IA_Sniper.IA_Sniper")))

(event EventBeginPlay)

(event EventOnGameOver
  (|CallParentFunction)
  (Development|PrintString "Game Over!!!"))

(event EventOnUsingGrenade
  (params (isGrenade :type Boolean))
  (Development|PrintString (Utilities|String|ToString(Boolean) isGrenade)))

(fn ConstructionScript)